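; BP_WinCondition is a victory pickup that triggers the win when the player touches it.
; A timeline started on BeginPlay moves its flipbook vertically between 0 and 50 units for an up-and-down motion.
; When BP_Player overlaps the box, it finds the top-level MainGameWidget by class search, calls Victory on it, plays a sound and destroys itself.
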(event OnComponentBeginOverlap(Box)
  (params (OverlappedComponent :type Primitive%20Component%20Object%20Reference) (OtherActor :type Actor%20Object%20Reference) (OtherComp :type Primitive%20Component%20Object%20Reference) (OtherBodyIndex :type Integer) (bFromSweep :type Boolean) (SweepResult :type Hit%20Result%20Structure%20%28by%20ref%29))
  (Utilities|Casting|CastToBP_Player OtherActor)
  (bind _foundwidgets (Widget|GetAllWidgetsOfClass "/Game/Blueprints/UI/MainGameWidget.MainGameWidget_C" true))
  (bind _asmain_game_widget (Utilities|Casting|CastToMainGameWidget (Utilities|Array|Get(acopy) _foundwidgets)))
  (Default|Victory _asmain_game_widget)
  (Audio|PlaySound2D "/Game/Music_SFX/Jump1.Jump1" 1.0 1.0 0.0 0 0)
  (Actor|DestroyActor))

(event EventBeginPlay
  (bind _paperflipbook (Variables|Default|GetPaperFlipbook))
  (bind _relativelocation (Variables|/Script/Engine.SceneComponent|GetRelativeLocation _paperflipbook))
  (bind _newtrack_0 (Timeline|UpDown Play)
    (:Update
      (Transformation|SetRelativeLocation _paperflipbook (Math|Vector|MakeVector (.x _relativelocation) (.y _relativelocation) (Math|Float|Lerp 0.0 5e+01 _newtrack_0)) false false))))

(fn ConstructionScript)