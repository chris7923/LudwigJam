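; Spline path actor that constrains the player character's movement to a spline.
; On BeginPlay it registers itself as the player's current spline and snaps the capsule to the closest spline point.
; Each Tick it re-projects the capsule's X and Y onto the spline while preserving Z, leaving vertical movement free.
; It also sets the player's yaw to face the path's Billboard component every frame.
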(event EventBeginPlay
  (bind _asbp_player (Utilities|Casting|CastToBP_Player (Game|GetPlayerCharacter 0)))
  (bind _output_get (Variables|Default|SetPlayerRef _asbp_player))
  (Variables|/Game/Blueprints/BP_Player.BP_Player_C|SetCurrentSpline _output_get self)
  (Transformation|SetWorldLocation (Variables|/Script/Engine.Character|GetCapsuleComponent _output_get) (Spline|FindLocationClosesttoWorldLocation (Variables|Default|GetSpline) (Transformation|GetWorldLocation (Variables|/Script/Engine.Character|GetCapsuleComponent (Variables|Default|GetPlayerRef))) "World") false false))

(event EventTick
  (params (DeltaSeconds :type Float%20%28single-precision%29))
  (bind _spline (Variables|Default|GetSpline))
  (bind _playerref (Variables|Default|GetPlayerRef))
  (bind _capsulecomponent (Variables|/Script/Engine.Character|GetCapsuleComponent _playerref))
  (bind _returnvalue (Transformation|GetWorldLocation _capsulecomponent))
  (bind _returnvalue_2 (Spline|FindLocationClosesttoWorldLocation _spline _returnvalue "World"))
  (Transformation|SetWorldLocation (Variables|/Script/Engine.Character|GetCapsuleComponent _playerref) (Math|Vector|MakeVector (.x _returnvalue_2) (.y _returnvalue_2) (.Z (Math|Vector|BreakVector _returnvalue))) false false)
  (Transformation|SetActorRotation _playerref (Math|Rotator|MakeRotator 0.0 0.0 (.yaw (Math|Rotator|FindLookatRotation _returnvalue (Transformation|GetWorldLocation (Variables|Default|GetBillboard)))))))

(fn ConstructionScript)