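; Player frog character that leaps toward the mouse cursor using charged jumps, with 8-direction flipbook animation.
; Tick aims the Sphere at the cursor, or pushes the character along -Y while InWater.
; Holding left mouse charges JumpMultiplier via a timeline; release launches along the Sphere's forward vector, and Q cancels.
; Cursor yaw picks Direction for idle/jump flipbooks; R resets position, and ZoomOut lengthens the camera boom.
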(event Custom|JumpEvent
  (bind _returnvalue (Game|GetPlayerController 0))
  (bind _returnvalue_2 (Transformation|GetActorLocation))
  (bind _array (Utilities|Array|MakeArray "ObjectTypeQuery1" "ObjectTypeQuery2" "ObjectTypeQuery3" "ObjectTypeQuery4"))
  (bind _sphere (Variables|Default|GetSphere))
  (bind _jumpmultiplier (Variables|Default|GetJumpMultiplier))
  (bind _maxjump (Variables|Default|GetMaxJump))
  (bind _returnvalue_3 (Math|Vector|GetForwardVector _sphere))
  (bind _hitresult (Class|PlayerController|GetHitResultUnderCursorforObjects _returnvalue _array true))
  (bind _returnvalue_4 (* _maxjump _jumpmultiplier))
  (bind _location (Collision|BreakHitResult _hitresult))
  (bind _returnvalue_5 (Math|Rotator|FindLookatRotation _returnvalue_2 _location))
  (bind _yaw (Math|Rotator|BreakRotator _returnvalue_5))
  (Variables|Default|SetisGrounded false)
  (Character|LaunchCharacter (Math|Vector|MakeVector (* (.x _returnvalue_3) _returnvalue_4) (* (.y _returnvalue_3) _returnvalue_4) _returnvalue_4) true true)
  (Audio|PlaySound2D "/Game/Music_SFX/JumpFrog.JumpFrog" 1.0 1.0 0.0 0 0)
  (if (> _yaw 112.5)
    (Variables|Default|SetDirection "NewEnumerator6")
    (elif (> _yaw 67.5)
      (Variables|Default|SetDirection "NewEnumerator3")
      (elif (> _yaw 22.5)
        (Variables|Default|SetDirection "NewEnumerator4")
        (elif (> _yaw -22.5)
          (Variables|Default|SetDirection "NewEnumerator0")
          (elif (> _yaw -67.5)
            (Variables|Default|SetDirection "NewEnumerator5")
            (elif (> _yaw -112.5)
              (Variables|Default|SetDirection "NewEnumerator2")
              (elif (> _yaw -157.5)
                (Variables|Default|SetDirection "NewEnumerator7")
                (elif (> _yaw -181.0)
                  (Variables|Default|SetDirection "NewEnumerator1")
                  (else
                    (Variables|Default|SetDirection "NewEnumerator6"))))))))))
  (CallFunction|AnimationStateMachine false false (Variables|Default|GetDirection)))

(event Custom|ZoomOut
  (bind _zoom (Timeline|Zoom Play)
    (:Update
      (Variables|/Script/Engine.SpringArmComponent|SetTargetArmLength (Variables|Default|GetSpringArm) (Math|Float|Lerp 6e+02 1.1e+03 _zoom)))))

(event EventTick
  (params (DeltaSeconds :type Float%20%28single-precision%29))
  (if (not (Variables|Default|GetinMainMenu))
    (if (Variables|Default|GetinWater)
      (Pawn|Input|AddMovementInput "0.000000,-1.000000, 0" 1.0 false)
      (else
        (Transformation|SetRelativeRotation (Variables|Default|GetSphere) (Math|Rotator|MakeRotator 0.0 0.0 (.Yaw (Math|Rotator|BreakRotator (Math|Rotator|FindLookatRotation (Transformation|GetActorLocation) (.Location (Collision|BreakHitResult (.HitResult (Class|PlayerController|GetHitResultUnderCursorforObjects (Game|GetPlayerController 0) (Utilities|Array|MakeArray "ObjectTypeQuery1" "ObjectTypeQuery2" "ObjectTypeQuery3" "ObjectTypeQuery4") true)))))))) false false)))))

(event EventOnLanded
  (params (Hit :type Hit%20Result%20Structure%20%28by%20ref%29))
  (Variables|Default|SetisGrounded true)
  (CallFunction|AnimationStateMachine false true (Variables|Default|GetDirection)))

(event EventBeginPlay
  (CallFunction|AnimationStateMachine false true "NewEnumerator1")
  (Variables|/Script/Engine.SpringArmComponent|SetTargetArmLength (Variables|Default|GetSpringArm) 6e+02))

(event Input|KeyboardEvents|R
  (params (Key :type Key%20Structure :default "None"))
  (:Pressed
    (Transformation|SetActorLocation "0,-300.000000,100.000000" false false)))

(event Input|MouseEvents|LeftMouseButton
  (params (Key :type Key%20Structure :default "None"))
  (bind _isgrounded (Variables|Default|GetisGrounded))
  (bind _inwater (Variables|Default|GetinWater))
  (bind _inmainmenu (Variables|Default|GetinMainMenu))
  (bind _returnvalue (not _inmainmenu))
  (bind _returnvalue_2 (not _inwater))
  (:Pressed
    (if (Math|Boolean|ANDBoolean _isgrounded _returnvalue_2 _returnvalue)
      (bind _multiplier (Timeline|JumpTimeline PlayFromStart)
        (:Update
          (bind _output_get (Variables|Default|SetJumpMultiplier _multiplier))
          (Development|PrintString (Utilities|String|ToString(Float) _output_get))))))
  (:Released
    (if (Math|Boolean|ANDBoolean _isgrounded _returnvalue_2 _returnvalue)
      (CallFunction|JumpEvent)
      (Timeline|JumpTimeline Stop))))

(event Input|KeyboardEvents|Q
  (params (Key :type Key%20Structure :default "None"))
  (:Pressed
    (Variables|Default|SetJumpMultiplier 0.0)
    (bind _multiplier (Timeline|JumpTimeline Stop)
      (:Update
        (bind _output_get (Variables|Default|SetJumpMultiplier _multiplier))
        (Development|PrintString (Utilities|String|ToString(Float) _output_get))))))

(fn ConstructionScript)

(fn AnimationStateMachine
  (params (Looping :type Boolean) (isIdle :type Boolean) (Direction :type Directions%20Enum :default "NewEnumerator0"))
  (bind _peepojump (Variables|Default|GetPeepoJump))
  (bind _peepojump_2 (Variables|Default|GetPeepoJump))
  (Components|Timeline|SetLooping (Variables|Default|GetPeepoJump) Looping)
  (if isIdle
    (Sprite|SetFlipbook _peepojump (Utilities|Select :Index Direction :NewEnumerator0 "/Game/Asstes/2DAssets/IdleUp.IdleUp" :NewEnumerator1 "/Game/Asstes/2DAssets/IdleDown.IdleDown" :NewEnumerator3 "/Game/Asstes/2DAssets/IdleRight.IdleRight" :NewEnumerator2 "/Game/Asstes/2DAssets/IdleLeft.IdleLeft" :NewEnumerator4 "/Game/Asstes/2DAssets/IdleUpRight.IdleUpRight" :NewEnumerator5 "/Game/Asstes/2DAssets/IdleUpLeft.IdleUpLeft" :NewEnumerator6 "/Game/Asstes/2DAssets/IdleDownRight.IdleDownRight" :NewEnumerator7 "/Game/Asstes/2DAssets/IdleDownLeft.IdleDownLeft"))
    (Components|Timeline|PlayfromStart _peepojump)
    (else
      (Sprite|SetFlipbook _peepojump_2 (Utilities|Select :Index Direction :NewEnumerator0 "/Game/Asstes/2DAssets/JumpUp.JumpUp" :NewEnumerator1 "/Game/Asstes/2DAssets/JumpDown.JumpDown" :NewEnumerator3 "/Game/Asstes/2DAssets/JumpRight.JumpRight" :NewEnumerator2 "/Game/Asstes/2DAssets/JumpLeft.JumpLeft" :NewEnumerator4 "/Game/Asstes/2DAssets/JumpUpRight.JumpUpRight" :NewEnumerator5 "/Game/Asstes/2DAssets/JumpUpLeft.JumpUpLeft" :NewEnumerator6 "/Game/Asstes/2DAssets/JumpDownRight.JumpDownRight" :NewEnumerator7 "/Game/Asstes/2DAssets/JumpDownLeft.JumpDownLeft"))
      (Components|Timeline|PlayfromStart _peepojump_2))))